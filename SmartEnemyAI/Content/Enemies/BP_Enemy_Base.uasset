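; BP_Enemy_Base is an enemy base Blueprint that provides sword wielding and a melee attack.
; WieldSword spawns a BP_Sword, snaps it to the right-hand socket on the mesh and flags the enemy as wielding it.
; Attack plays a sword slash montage and calls OnAttackEnd whether the montage completes or is interrupted.
; GetPatrolRoute is an empty stub, and BeginPlay and the construction script do nothing.
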(event `self.ReceiveBeginPlay`)

(event `Attack`
  (`|PlayMontage` (`self.Mesh`) "/Game/Animations/Sword_Slash_Montage.Sword_Slash_Montage"
    (:`OnCompleted`
      _)
    (:`OnInterrupted`
      _))
  (`self.OnAttackEnd`))

(event `WieldSword`
  (bind _returnvalue (`|SpawnActorFromClass` "/Game/Weapons/BP_Sword.BP_Sword_C" (`self.GetTransform`) "Undefined" "OverrideRootScale" null null))
  (`self.K2_AttachToComponent` _returnvalue (`self.Mesh`) "hand_r_sword_socket" "SnapToTarget" "SnapToTarget" "SnapToTarget" true)
  (set `self.IsWieldingSword` true))

(fn `GetPatrolRoute`
  (returns (PatrolRoute :type "/Game/Enemies/AI/BP_PatrolRoute Object Reference"))
  (return null))

(fn `UserConstructionScript`)